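; BP_FloatArea is a side-scroller volume that makes the player character float inside its Cylinder.
; Beginning overlap with the Cylinder calls StartFloat on the 2DSideScrollerCharacter.
; Tick polls the Cylinder to set the character's IsInFloatingArea flag on entry and clear it on exit, using StartJudge to track occupancy.
; The construction script snaps the actor to Y=0 to keep it on the 2D plane.
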(event OnComponentBeginOverlap(Cylinder)
  (params (OverlappedComponent :type Primitive%20Component%20Object%20Reference) (OtherActor :type Actor%20Object%20Reference) (OtherComp :type Primitive%20Component%20Object%20Reference) (OtherBodyIndex :type Integer) (bFromSweep :type Boolean) (SweepResult :type Hit%20Result%20Structure%20%28by%20ref%29))
  (bind _as2dside_scroller_character (Utilities|Casting|CastTo2DSideScrollerCharacter OtherActor))
  (Utilities|IsValid _as2dside_scroller_character
    (:Is%20Valid
      (Default|StartFloat _as2dside_scroller_character))))

(event EventBeginPlay)

(event Collision|EventActorBeginOverlap
  (params (OtherActor :type Actor%20Object%20Reference)))

(event EventTick
  (params (DeltaSeconds :type Float%20%28single-precision%29))
  (bind _cylinder (Variables|Default|GetCylinder))
  (bind _overlappingactors (Collision|GetOverlappingActors _cylinder "/Game/2DSideScrollerBP/Blueprints/2DSideScrollerCharacter.2DSideScrollerCharacter_C" :!class /Script/Engine.PrimitiveComponent))
  (bind _output (Utilities|Array|Get(acopy) _overlappingactors))
  (Utilities|FlowControl|Sequence
    (:then_0
      (if (not (Variables|Default|GetbStartJudge))
        (Utilities|IsValid _output
          (:Is%20Valid
            (Variables|Default|SetbStartJudge true)
            (bind _output_get (Variables|Default|SetPlayerCharacter _output))
            (bind _as2dside_scroller_character (Utilities|Casting|CastTo2DSideScrollerCharacter _output_get))
            (Variables|/Game/2DSideScrollerBP/Blueprints/2DSideScrollerCharacter.2DSideScrollerCharacter_C|SetbIsInFloatingArea? _as2dside_scroller_character true)))))
    (:then_1
      (if (Variables|Default|GetbStartJudge)
        (Utilities|IsValid (Variables|Default|GetPlayerCharacter)
          (:Is%20Valid
            (bind _as2dside_scroller_character_2 (Utilities|Casting|CastTo2DSideScrollerCharacter (Variables|Default|GetPlayerCharacter)))
            (if (not (Collision|IsOverlappingActor (Variables|Default|GetCylinder) (Variables|Default|GetPlayerCharacter) :!class /Script/Engine.PrimitiveComponent))
              (Variables|/Game/2DSideScrollerBP/Blueprints/2DSideScrollerCharacter.2DSideScrollerCharacter_C|SetbIsInFloatingArea? _as2dside_scroller_character_2 false)
              (Variables|Default|SetbStartJudge false))))))))

(fn ConstructionScript
  (bind _returnvalue (Transformation|GetActorLocation))
  (Transformation|SetActorLocation (Math|Vector|MakeVector (.x _returnvalue) 0.0 (.z _returnvalue)) false false))