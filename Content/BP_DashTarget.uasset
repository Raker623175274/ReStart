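; BP_DashTarget is a target actor, named for dashing, with a cylinder that travels along its spline.
; StartMove plays the Move timeline from the start, mapping its Alpha to distance along the spline to set the cylinder's local position.
; The construction script locks the actor to the Y=0 plane, sizes the flattened cylinder from PointScale and applies PlayRate to the timeline.
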(event Custom|StartMove
  (bind _spline (Variables|Default|GetSpline))
  (bind _alpha (Timeline|Move PlayFromStart)
    (:Update
      (Transformation|SetRelativeLocation (Variables|Default|GetCylinder) (Spline|GetLocationatDistanceAlongSpline _spline (* (Spline|GetSplineLength _spline) _alpha) "Local") false false))))

(fn ConstructionScript
  (bind _returnvalue (Transformation|GetActorLocation))
  (bind _pointscale (Variables|Default|GetPointScale))
  (Transformation|SetActorLocation (Math|Vector|MakeVector (.x _returnvalue) 0.0 (.z _returnvalue)) false false)
  (Transformation|SetRelativeScale3D (Variables|Default|GetCylinder) (Math|Vector|MakeVector _pointscale _pointscale 0.25))
  (Components|Timeline|SetPlayRate (Variables|Default|GetMove) (Variables|Default|GetPlayRate)))