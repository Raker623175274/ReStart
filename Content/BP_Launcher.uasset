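; BP_Launcher is a launcher for a 2D side-scroller that registers itself with the player character it overlaps.
; Each tick it checks for overlap with player 0 and, while overlapping, sets itself as that character's CurrentLauncher; the launch itself is not performed here.
; The construction script snaps the actor to Y=0 to keep it on the gameplay plane and picks its jumper sprite from CanLaunch.
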(event EventTick
  (params (DeltaSeconds :type Float%20%28single-precision%29))
  (bind _returnvalue (Game|GetPlayerCharacter 0))
  (if (Collision|IsOverlappingActor _returnvalue :!class /Script/Engine.Actor)
    (bind _as2dside_scroller_character (Utilities|Casting|CastTo2DSideScrollerCharacter _returnvalue))
    (Utilities|IsValid _as2dside_scroller_character
      (:Is%20Valid
        (Variables|/Game/2DSideScrollerBP/Blueprints/2DSideScrollerCharacter.2DSideScrollerCharacter_C|SetCurrentLauncher _as2dside_scroller_character self)))))

(fn ConstructionScript
  (bind _returnvalue (Transformation|GetActorLocation))
  (bind _spritesheet_jumper__49 (Variables|Default|Getspritesheet_jumper__49))
  (Utilities|FlowControl|Sequence
    (:then_0
      (Transformation|SetActorLocation (Math|Vector|MakeVector (.x _returnvalue) 0.0 (.z _returnvalue)) false false))
    (:then_1
      (if (Variables|Default|GetbCanLaunch?)
        (Rendering|Components|Sprite|SetSprite _spritesheet_jumper__49 "/Game/ArtAssets/Environment/Sprites/spritesheet_jumper__49.spritesheet_jumper__49")
        (else
          (Rendering|Components|Sprite|SetSprite _spritesheet_jumper__49 "/Game/ArtAssets/Environment/Sprites/spritesheet_jumper__41.spritesheet_jumper__41"))))))