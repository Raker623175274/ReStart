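; BP_MoveableBaord is a moving board for the 2D side scroller that moves when the player character's MoveableBoardsStartMoving event fires.
; A Move timeline, gated by CanMove against retriggering, lerps between the first two spline points.
; Each update adds that result to the sprite as a cumulative local offset rather than setting its position.
; Construction snaps the actor to Y=0; spline-length speed scaling is present but never runs.
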(event Custom|StartMove
  (bind _spline (Variables|Default|GetSpline))
  (if (Variables|Default|GetbCanMove?)
    (Variables|Default|SetbCanMove? false)
    (bind _alpha (Timeline|Move PlayFromStart)
      (:Update
        (Transformation|AddLocalOffset (Variables|Default|Getspritesheet_jumper__22) (Math|Vector|Lerp(Vector) (Spline|GetLocationatSplinePoint _spline 0 "Local") (Spline|GetLocationatSplinePoint _spline 1 "Local") _alpha) false false))
      (:Finished
        (Variables|Default|SetbCanMove? true)))))

(event EventBeginPlay
  (bind _as2dside_scroller_character (Utilities|Casting|CastTo2DSideScrollerCharacter (Game|GetPlayerCharacter 0)))
  (Utilities|IsValid _as2dside_scroller_character
    (:Is%20Valid
      (EventDispatchers|BindEventtoMoveableBoardsStartMoving _as2dside_scroller_character (delegate Custom|StartMove)))))

(fn ConstructionScript
  (bind _returnvalue (Transformation|GetActorLocation))
  (Transformation|SetActorLocation (Math|Vector|MakeVector (.x _returnvalue) 0.0 (.z _returnvalue)) false false))