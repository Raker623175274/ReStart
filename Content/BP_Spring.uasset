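; BP_Spring is a side-scroller spring pad that launches the player character along its arrow direction.
; Each tick it checks the player's overlap with its box, firing once per entry: it zeroes velocity, applies a velocity-change impulse, and ends and resets dash and launch state.
; The flipbook switches to a rebound animation, then returns to idle at a set frame.
; The construction script pins the actor to Y=0.
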(event EventBeginPlay)

(event EventTick
  (params (DeltaSeconds :type Float%20%28single-precision%29))
  (Utilities|FlowControl|Sequence
    (:then_0
      (bind _as2dside_scroller_character (Utilities|Casting|CastTo2DSideScrollerCharacter (Game|GetPlayerCharacter 0)))
      (Utilities|IsValid _as2dside_scroller_character
        (:Is%20Valid
          (if (Collision|IsOverlappingActor (Variables|Default|GetBox) _as2dside_scroller_character :!class /Script/Engine.PrimitiveComponent)
            (Utilities|FlowControl|DoOnce false :!label _label
              (:Completed
                (Utilities|FlowControl|Sequence
                  (:then_0
                    (Variables|/Script/Engine.MovementComponent|SetVelocity (Variables|/Script/Engine.Character|GetCharacterMovement _as2dside_scroller_character) "0, 0, 0")
                    (Physics|AddImpulse (Variables|/Script/Engine.Character|GetCharacterMovement _as2dside_scroller_character) (* (Math|Vector|GetForwardVector (Variables|Default|GetArrow)) (Variables|Default|GetImpulse)) true)
                    (Utilities|FlowControl|Sequence
                      (:then_0
                        (Default|EndDash _as2dside_scroller_character)
                        (Default|EndLaunch _as2dside_scroller_character))
                      (:then_1
                        (Default|ResetDash _as2dside_scroller_character))))
                  (:then_1
                    (Sprite|SetFlipbook (Variables|Default|GetPaperFlipbook) "/Game/ArtAssets/Environment/Sprites/Anim_SpringRebound.Anim_SpringRebound")
                    (Variables|Default|SetbRebound true)))))
            (else
              (goto _label Reset))))))
    (:then_1
      ;[1 1 1] Set Flipbook
      (if (Variables|Default|GetbRebound)
        (if (== (Class|PaperFlipbookComponent|GetPlaybackPositioninFrames (Variables|Default|GetPaperFlipbook)) 4)
          (Sprite|SetFlipbook (Variables|Default|GetPaperFlipbook) "/Game/ArtAssets/Environment/Sprites/Anim_Spring.Anim_Spring")
          (Variables|Default|SetbRebound false))))))

(fn ConstructionScript
  (bind _returnvalue (Transformation|GetActorLocation))
  (Transformation|SetActorLocation (Math|Vector|MakeVector (.x _returnvalue) 0.0 (.z _returnvalue)) false false))