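; Moveable board for a 2D side-scroller that slides a jumper sprite between two spline points and exposes a launch velocity while moving.
; StartMove, gated by CanMove, plays a timeline that lerps the sprite's position and re-arms on finish.
; A timeline track sets Moving and HoldJumpAccelerateSpeed along the travel direction with upward bias, clearing both above a threshold.
; Construction pins Y to zero; the character event binding and length-based time dilation are disconnected.
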(event Custom|StartMove
  (bind _spline (Variables|Default|GetSpline))
  (bind _returnvalue (Spline|GetLocationatSplinePoint _spline 1 "World"))
  (bind _returnvalue_2 (Spline|GetLocationatSplinePoint _spline 0 "World"))
  (if (Variables|Default|GetbCanMove?)
    (Variables|Default|SetbCanMove? false)
    (bind (_direction _alpha _setholdacceleratespeed) (Timeline|Move PlayFromStart)
      (:Update
        (Transformation|SetWorldLocation (Variables|Default|Getspritesheet_jumper__22) (Math|Vector|Lerp(Vector) _returnvalue_2 _returnvalue _alpha) false false)
        (Math|Float|CompareFloat _setholdacceleratespeed 1.0
          (:>
            (Variables|Default|SetbMoving? false)
            (Variables|Default|SetHoldJumpAccelerateSpeed "0, 0, 0"))
          (:==
            (Variables|Default|SetHoldJumpAccelerateSpeed (* (Math|Vector|Normalize (+ (Math|Vector|Normalize (- _returnvalue _returnvalue_2)) "0, 0,0.800000")) (Math|Float|Lerp 1.3e+03 1.6e+03 (Math|Float|Clamp(Float) _setholdacceleratespeed))) :!label _label)
            (Variables|Default|SetbMoving? true))
          (:<
            (goto _label))))
      (:Finished
        (Variables|Default|SetbCanMove? true)))))

(event EventBeginPlay)

(fn ConstructionScript
  (bind _returnvalue (Transformation|GetActorLocation))
  (Transformation|SetActorLocation (Math|Vector|MakeVector (.x _returnvalue) 0.0 (.z _returnvalue)) false false))