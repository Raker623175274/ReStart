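; Teleport point for a 2D side-scroller that launches a dashing player a set distance along their control direction.
; Tick polls the cylinder for player overlap; during Dash it ends the dash, moves the player with a swept SetActorLocation via a self-resetting DoOnce, then resets the dash.
; A separate Teleport event repeats the move without overlap or state checks.
; The construction script pins the actor to Y=0 and sizes the cylinder from PointScale.
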(event Custom|Teleport
  (bind _returnvalue (Game|GetPlayerCharacter 0))
  (Utilities|IsValid _returnvalue
    (:Is%20Valid
      (bind _as2dside_scroller_character (Utilities|Casting|CastTo2DSideScrollerCharacter _returnvalue))
      (Transformation|SetActorLocation _as2dside_scroller_character (+ (Transformation|GetActorLocation _returnvalue) (* (Default|CalculateControlDirection _as2dside_scroller_character) (Variables|Default|GetTeleportLength))) true false)
      (Default|ResetDash _as2dside_scroller_character))))

(event EventTick
  (params (DeltaSeconds :type Float%20%28single-precision%29))
  (bind _returnvalue (Game|GetPlayerCharacter 0))
  (if (Collision|IsOverlappingActor (Variables|Default|GetCylinder) (Game|GetPlayerCharacter 0) :!class /Script/Engine.PrimitiveComponent)
    (bind _as2dside_scroller_character (Utilities|Casting|CastTo2DSideScrollerCharacter (Game|GetPlayerCharacter 0)))
    (switch Utilities|FlowControl|Switch|SwitchonEnum_CharacterStates (Variables|/Game/2DSideScrollerBP/Blueprints/2DSideScrollerCharacter.2DSideScrollerCharacter_C|GetCharacterStates _as2dside_scroller_character)
      (:NewEnumerator0
        (Default|EndDash _as2dside_scroller_character false 1.5e+03)
        (Utilities|FlowControl|DoOnce false :!label _label
          (:Completed
            (Transformation|SetActorLocation _returnvalue (+ (Transformation|GetActorLocation _returnvalue) (* (Default|CalculateControlDirection _as2dside_scroller_character) (Variables|Default|GetTeleportLength))) true false)
            (Default|ResetDash _as2dside_scroller_character)
            (goto _label Reset)))))))

(fn ConstructionScript
  (bind _returnvalue (Transformation|GetActorLocation))
  (bind _pointscale (Variables|Default|GetPointScale))
  (Transformation|SetActorLocation (Math|Vector|MakeVector (.x _returnvalue) 0.0 (.z _returnvalue)) false false)
  (Transformation|SetRelativeScale3D (Variables|Default|GetCylinder) (Math|Vector|MakeVector _pointscale _pointscale 0.25)))