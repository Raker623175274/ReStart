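; BP_TeleportPoint2 is one end of a linked teleporter pair that moves a dashing 2D side-scroller character to the other point.
; Cylinder overlap disables both points before checking the character's state, re-enabling them 0.5 seconds after a teleport only, so other overlaps leave them disabled.
; Teleporting also retimes the character's Dash timeline.
; The construction script pins the actor to Y=0 and sizes the cylinder from PointScale.
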(event OnComponentBeginOverlap(Cylinder)
  (params (OverlappedComponent :type Primitive%20Component%20Object%20Reference) (OtherActor :type Actor%20Object%20Reference) (OtherComp :type Primitive%20Component%20Object%20Reference) (OtherBodyIndex :type Integer) (bFromSweep :type Boolean) (SweepResult :type Hit%20Result%20Structure%20%28by%20ref%29))
  (if (Variables|Default|GetbCanTeleport?)
    (Variables|Default|SetbCanTeleport? false)
    (Variables|BP_TeleportPoint2_C|SetbCanTeleport? (Variables|Default|GetTheOtherTeleportPoint) false)
    (bind _as2dside_scroller_character (Utilities|Casting|CastTo2DSideScrollerCharacter OtherActor))
    (Utilities|IsValid _as2dside_scroller_character
      (:Is%20Valid
        (switch Utilities|FlowControl|Switch|SwitchonEnum_CharacterStates (Variables|/Game/2DSideScrollerBP/Blueprints/2DSideScrollerCharacter.2DSideScrollerCharacter_C|GetCharacterStates _as2dside_scroller_character)
          (:NewEnumerator0
            (Transformation|SetActorLocation _as2dside_scroller_character (Transformation|GetActorLocation (Variables|Default|GetTheOtherTeleportPoint)) false true)
            (Components|Timeline|SetNewTime (Variables|/Game/2DSideScrollerBP/Blueprints/2DSideScrollerCharacter.2DSideScrollerCharacter_C|GetDash _as2dside_scroller_character) 0.1)
            (Utilities|FlowControl|Delay 0.5)
            (Variables|Default|SetbCanTeleport? true)
            (Variables|BP_TeleportPoint2_C|SetbCanTeleport? (Variables|Default|GetTheOtherTeleportPoint) true)
            (Development|PrintString "Hello")))))))

(fn ConstructionScript
  (bind _returnvalue (Transformation|GetActorLocation))
  (bind _pointscale (Variables|Default|GetPointScale))
  (Transformation|SetActorLocation (Math|Vector|MakeVector (.x _returnvalue) 0.0 (.z _returnvalue)) false false)
  (Transformation|SetRelativeScale3D (Variables|Default|GetCylinder) (Math|Vector|MakeVector _pointscale _pointscale 0.25)))