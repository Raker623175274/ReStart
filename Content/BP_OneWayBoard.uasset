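; BP_OneWayBoard is a one-way platform for a 2D side-scroller that the player can pass through from below and stand on from above.
; Every tick it compares the player character's height to its own and enables the Paper sprite's collision only when the player is above it by more than the scaled capsule half-height plus a small margin.
; The construction script snaps the board to zero on the Y axis, keeping it on the gameplay plane.
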(event EventTick
  (params (DeltaSeconds :type Float%20%28single-precision%29))
  (bind _returnvalue (Game|GetPlayerCharacter 0))
  (bind _papersprite (Variables|Default|GetPaperSprite))
  (bind _as2dside_scroller_character (Utilities|Casting|CastTo2DSideScrollerCharacter _returnvalue))
  (Utilities|IsValid _as2dside_scroller_character
    (:Is%20Valid
      (if (> (- (.z (Transformation|GetActorLocation _returnvalue)) (.z (Transformation|GetActorLocation))) (+ (Components|Capsule|GetScaledCapsuleHalfHeight (Variables|/Script/Engine.Character|GetCapsuleComponent _as2dside_scroller_character)) 1e+01))
        (Collision|SetCollisionEnabled _papersprite "QueryAndPhysics")
        (else
          (Collision|SetCollisionEnabled _papersprite "NoCollision"))))))

(fn ConstructionScript
  (bind _returnvalue (Transformation|GetActorLocation))
  (bind (_x _y _z) (Math|Vector|BreakVector _returnvalue))
  (Transformation|SetActorLocation (Math|Vector|MakeVector _x 0.0 _z) false false))