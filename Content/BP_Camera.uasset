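; BP_Camera is a camera actor for a side-view game that follows the player character along X and Z while holding Y at its start location.
; Each tick it moves to the player's clamped X and Z, with per-axis toggles that otherwise keep the start coordinate.
; The construction script snaps it to StartLocation.
; A ChangeCamera event blends player 0's view to a given target with a short cubic blend.
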(event Custom|ChangeCamera
  (params (NewParam :type BP%20Camera%20Object%20Reference))
  (Game|Player|SetViewTargetwithBlend (Game|GetPlayerController 0) NewParam 0.5 "VTBlend_Cubic" 1.0 false))

(event EventTick
  (params (DeltaSeconds :type Float%20%28single-precision%29))
  (bind _returnvalue (Game|GetPlayerCharacter 0))
  (bind _startlocation (Variables|Default|GetStartLocation))
  (bind _returnvalue_2 (Transformation|GetActorLocation _returnvalue))
  (bind (_x _y _z) (Math|Vector|BreakVector _returnvalue_2))
  (Utilities|FlowControl|Sequence
    (:then_0
      (Transformation|SetActorLocation (Math|Vector|MakeVector (select (Variables|Default|GetbCanMoveRight?) (Math|Float|Clamp(Float) _x (Variables|Default|GetRightXMin) (Variables|Default|GetRightXMax)) (.x _startlocation)) (.y _startlocation) (select (Variables|Default|GetbCanMoveUp?) (Math|Float|Clamp(Float) _z (Variables|Default|GetUpZMin) (Variables|Default|GetUpZMax)) (.z _startlocation))) false false))))

(fn ConstructionScript
  (Transformation|SetActorLocation (Variables|Default|GetStartLocation) false false))