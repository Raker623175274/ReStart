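; BP_SavePoint is a side-scroller checkpoint trigger that updates the character's respawn point and switches between two cameras.
; Tick compares its position with the player's on X or Z, chosen by RightLeftUpDown, to set the RightUp direction flag.
; On box overlap by the 2DSideScrollerCharacter, that flag selects which save point becomes RebornPoint and which way ChangeCamera runs between CameraLeftDown and CameraRightUp.
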(event OnComponentBeginOverlap(Box)
  (params (OverlappedComponent :type Primitive%20Component%20Object%20Reference) (OtherActor :type Actor%20Object%20Reference) (OtherComp :type Primitive%20Component%20Object%20Reference) (OtherBodyIndex :type Integer) (bFromSweep :type Boolean) (SweepResult :type Hit%20Result%20Structure%20%28by%20ref%29))
  (bind _savepointright_up (Variables|Default|GetSavePointRight/Up))
  (bind _savepointleft_down (Variables|Default|GetSavePointLeft/Down))
  (bind _as2dside_scroller_character (Utilities|Casting|CastTo2DSideScrollerCharacter OtherActor))
  (Utilities|IsValid _as2dside_scroller_character
    (:Is%20Valid
      (if (Variables|Default|GetbRight/Up?)
        (Utilities|FlowControl|Sequence
          (:then_0
            (Utilities|IsValid _savepointright_up
              (:Is%20Valid
                (Variables|/Game/2DSideScrollerBP/Blueprints/2DSideScrollerCharacter.2DSideScrollerCharacter_C|SetRebornPoint _as2dside_scroller_character _savepointright_up))))
          (:then_1
            (Default|ChangeCamera (Variables|Default|GetCameraLeft/Down) (Variables|Default|GetCameraRight/Up))))
        (else
          (Utilities|FlowControl|Sequence
            (:then_0
              (Utilities|IsValid _savepointleft_down
                (:Is%20Valid
                  (Variables|/Game/2DSideScrollerBP/Blueprints/2DSideScrollerCharacter.2DSideScrollerCharacter_C|SetRebornPoint _as2dside_scroller_character _savepointleft_down))))
            (:then_1
              (Default|ChangeCamera (Variables|Default|GetCameraRight/Up) (Variables|Default|GetCameraLeft/Down)))))))))

(event EventTick
  (params (DeltaSeconds :type Float%20%28single-precision%29))
  (bind _returnvalue (Game|GetPlayerCharacter 0))
  (Utilities|FlowControl|Sequence
    (:then_0
      (if (Variables|Default|GetbRightLeft/UpDown?)
        (Utilities|IsValid _returnvalue
          (:Is%20Valid
            (Variables|Default|SetbRight/Up? (> (- (.x (Transformation|GetActorLocation)) (.x (Transformation|GetActorLocation _returnvalue))) 0.0))))
        (else
          (Utilities|IsValid _returnvalue
            (:Is%20Valid
              (Variables|Default|SetbRight/Up? (> (- (.z (Transformation|GetActorLocation)) (.z (Transformation|GetActorLocation _returnvalue))) 0.0)))))))))

(fn ConstructionScript)